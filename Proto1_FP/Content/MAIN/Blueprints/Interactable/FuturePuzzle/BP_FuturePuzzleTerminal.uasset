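; BP_FuturePuzzleTerminal is an interactable terminal for the Future puzzle.
; Overlapping its box shows a widget component, and leaving the box hides it.
; The Interact event creates the terminal screen widget for player 0, adds it to the viewport, shows the mouse cursor and switches input to UI-only, focused on that screen.
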(event OnComponentBeginOverlap(Box)
  (params (OverlappedComponent :type Primitive%20Component%20Object%20Reference) (OtherActor :type Actor%20Object%20Reference) (OtherComp :type Primitive%20Component%20Object%20Reference) (OtherBodyIndex :type Integer) (bFromSweep :type Boolean) (SweepResult :type Hit%20Result%20Structure%20%28by%20ref%29))
  ;[0.15 0.15 0.15 0.5] Interact
  (Rendering|SetVisibility (Variables|Default|GetWidget) true false))

(event OnComponentEndOverlap(Box)
  (params (OverlappedComponent :type Primitive%20Component%20Object%20Reference) (OtherActor :type Actor%20Object%20Reference) (OtherComp :type Primitive%20Component%20Object%20Reference) (OtherBodyIndex :type Integer))
  ;[0.15 0.15 0.15 0.5] Interact
  (Rendering|SetVisibility (Variables|Default|GetWidget) false false))

(event EventInteract
  (bind _returnvalue (Game|GetPlayerController 0))
  ;[0.15 0.15 0.15 0.5] Interaction: FuturePuzzle
  (bind _returnvalue_2 (UserInterface|CreateWidget "/Game/MAIN/Blueprints/Interactable/FuturePuzzle/WBP_FuturePuzzleTerminalScreen.WBP_FuturePuzzleTerminalScreen_C" (Game|GetPlayerController 0)))
  (UserInterface|Viewport|AddtoViewport _returnvalue_2 0)
  (Variables|/Script/Engine.PlayerController|SetbShowMouseCursor _returnvalue true)
  (Input|SetInputModeUIOnly _returnvalue _returnvalue_2 "DoNotLock" true))

(fn ConstructionScript)
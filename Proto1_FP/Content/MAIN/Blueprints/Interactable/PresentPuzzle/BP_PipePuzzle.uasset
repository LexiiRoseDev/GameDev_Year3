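; BP_PipePuzzle is an interactable that opens the pipe puzzle UI when the player is near it.
; It creates the WBP_PipePuzzle widget at BeginPlay and enables input when its box is overlapped.
; E toggles the widget through a FlipFlop, switching mouse cursor and input mode with it.
; Ending the overlap disables input and closes the widget, re-triggering the FlipFlop if open to keep the toggle in sync.
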(event OnComponentBeginOverlap(Box)
  (params (OverlappedComponent :type Primitive%20Component%20Object%20Reference) (OtherActor :type Actor%20Object%20Reference) (OtherComp :type Primitive%20Component%20Object%20Reference) (OtherBodyIndex :type Integer) (bFromSweep :type Boolean) (SweepResult :type Hit%20Result%20Structure%20%28by%20ref%29))
  (Input|EnableInput (Game|GetPlayerController 0)))

(event OnComponentEndOverlap(Box)
  (params (OverlappedComponent :type Primitive%20Component%20Object%20Reference) (OtherActor :type Actor%20Object%20Reference) (OtherComp :type Primitive%20Component%20Object%20Reference) (OtherBodyIndex :type Integer))
  (bind _returnvalue (Game|GetPlayerController 0))
  (Input|DisableInput _returnvalue 0)
  (if (stale _isa)
    (bind _isa (Utilities|FlowControl|FlipFlop)
      (:A
        (UserInterface|Viewport|AddtoViewport (stale EventBeginPlay _returnvalue) 0)
        (Variables|/Script/Engine.PlayerController|SetbShowMouseCursor _returnvalue true)
        (Input|SetInputModeGameandUI _returnvalue (stale EventBeginPlay _returnvalue) "DoNotLock" true false))
      (:B
        (Widget|RemovefromParent (stale EventBeginPlay _returnvalue) :!label _label)
        (Variables|/Script/Engine.PlayerController|SetbShowMouseCursor _returnvalue false)
        (Input|SetInputModeGameOnly _returnvalue false)))
    (else
      (goto _label))))

(event EventBeginPlay
  (bind _returnvalue (UserInterface|CreateWidget "/Game/MAIN/Blueprints/Interactable/PresentPuzzle/WBP_PipePuzzle.WBP_PipePuzzle_C")))

(event Input|KeyboardEvents|E
  (params (Key :type Key%20Structure :default "None"))
  (bind _returnvalue (Game|GetPlayerController 0))
  (:Pressed
    (bind _isa (Utilities|FlowControl|FlipFlop)
      (:A
        (UserInterface|Viewport|AddtoViewport (stale EventBeginPlay _returnvalue) 0)
        (Variables|/Script/Engine.PlayerController|SetbShowMouseCursor _returnvalue true)
        (Input|SetInputModeGameandUI _returnvalue (stale EventBeginPlay _returnvalue) "DoNotLock" true false))
      (:B
        (Widget|RemovefromParent (stale EventBeginPlay _returnvalue))
        (Variables|/Script/Engine.PlayerController|SetbShowMouseCursor _returnvalue false)
        (Input|SetInputModeGameOnly _returnvalue false)))))

(fn ConstructionScript)
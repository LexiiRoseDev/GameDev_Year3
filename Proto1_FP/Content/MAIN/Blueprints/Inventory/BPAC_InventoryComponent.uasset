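; Actor component that holds an inventory of numbered slots, built empty to a configured slot count on BeginPlay.
; AddItem takes the first empty slot, looks up the item ID in DT_InventoryItemData and adds the amount to the row's quantity.
; It then fills in the slot data, marked occupied, and broadcasts it through OnItemAdded.
; There is no stacking onto occupied slots, and a full inventory only prints the debug message.
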(event EventBeginPlay
  (CallFunction|InitialiseSlot))

(event EventTick
  (params (DeltaSeconds :type Float%20%28single-precision%29)))

(fn InitialiseSlot
  (for _index (range 0 (- (Variables|Default|GetNum%20of%20Inventory%20Slots) 1))
    (Utilities|Array|Add (Variables|Default|GetInventory%20Slots) (Utilities|Struct|MakeStruct_InventorySlotData true "(ItemID_2_13FB3FD34DA555D7B52B98A3806FFC06=\"\",ItemName_19_5E730D2F415036C3B82A70A63B05F8FD=\"\",ItemDescription_20_154C43234BE549D49194FC914A30B4B3=\"\",ItemIcon_21_A75AEF364A74BCA2CD8E9DAA7E1BD5B5=None,ItemBPClass_18_3A8E15BF4DAC4F8D04D04D9FF0C1F839=None,MaxQuantity_27_E1272CF1490E15C410EC918504269F75=0,CurrentQuantity_26_71091126455141E5EF030BA885AF31CD=0)" _index))))

(fn AddItem
  (params (Item%20ID :type String) (Amount :type Integer))
  (Development|PrintString (Utilities|String|Append "Item " Item%20ID " added to inventory"))
  (bind (_empty_slot_available _index) (CallFunction|CheckforEmptySlots))
  (if _empty_slot_available
    (bind _returnvalue (Utilities|GetDataTableRow "/Game/MAIN/Blueprints/Items/DT_InventoryItemData.DT_InventoryItemData" (Utilities|String|StringToName Item%20ID))
      (:then
        (bind _structout (Utilities|Struct|SetmembersinStruct_ItemData _returnvalue (+ (Utilities|Struct|BreakStruct_ItemData _returnvalue) Amount)))
        (bind _structout_2 (Utilities|Struct|SetmembersinStruct_InventorySlotData (Utilities|Array|Get(acopy) (Variables|Default|GetInventory%20Slots) _index) false _structout))
        (Default|CallOnItemAdded _structout_2)))))

(fn CheckforEmptySlots
  (bind (_array_element _array_index) (Utilities|Array|ForEachLoopwithBreak (Variables|Default|GetInventory%20Slots) :!label _label)
    (:LoopBody
      (if (.isEmpty (Utilities|Struct|BreakStruct_InventorySlotData _array_element))
        (Utilities|FlowControl|Sequence
          (:then_0
            (goto _label Break))
          (:then_1
            (return true _array_index)))))
    (:Completed
      (return false -1))))
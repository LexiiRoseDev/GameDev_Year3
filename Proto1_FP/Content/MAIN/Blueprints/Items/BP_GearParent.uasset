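; BP_GearParent is a base gear pickup that adds itself to the player's inventory on touch.
; On BeginPlay it looks up its ItemID in DT_InventoryItemData and caches the row in ItemDataStruct.
; When the first-person character overlaps its Sphere, it passes ItemID and Amount to that character's BPACInventoryComponent, then destroys itself.
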(event OnComponentBeginOverlap(Sphere)
  (params (OverlappedComponent :type Primitive%20Component%20Object%20Reference) (OtherActor :type Actor%20Object%20Reference) (OtherComp :type Primitive%20Component%20Object%20Reference) (OtherBodyIndex :type Integer) (bFromSweep :type Boolean) (SweepResult :type Hit%20Result%20Structure%20%28by%20ref%29))
  (bind _asbp_first_person_character (Utilities|Casting|CastToBP_FirstPersonCharacter OtherActor))
  (Default|AddItem (Variables|/Game/FirstPerson/Blueprints/BP_FirstPersonCharacter.BP_FirstPersonCharacter_C|GetBPAC_InventoryComponent _asbp_first_person_character) (Variables|Default|GetItem%20ID) (Variables|Default|GetAmount))
  (Actor|DestroyActor))

(event EventBeginPlay
  (CallFunction|InitialiseItemDataStructure))

(event Collision|EventActorBeginOverlap
  (params (OtherActor :type Actor%20Object%20Reference)))

(event EventTick
  (params (DeltaSeconds :type Float%20%28single-precision%29)))

(fn ConstructionScript)

(fn InitialiseItemDataStructure
  (bind _returnvalue (Utilities|GetDataTableRow "/Game/MAIN/Blueprints/Items/DT_InventoryItemData.DT_InventoryItemData" (Utilities|String|StringToName (Variables|Default|GetItem%20ID)))
    (:then
      (Variables|Default|SetItem%20Data%20Struct _returnvalue))))
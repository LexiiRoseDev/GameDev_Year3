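; BP_ClockPresent is an interactive present-time clock whose hands the player can turn and which opens menu widgets.
; A collision box shows a prompt widget and enables actor input while the player pawn is nearby.
; E opens the pipe puzzle or broken clock widget with mouse cursor, depending on the game instance's SecondRound flag.
; Left/Right step the hour hand and Up/Down the minute hand, with Shift for larger minute steps.
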(event OnComponentEndOverlap(Box)
  (params (OverlappedComponent :type Primitive%20Component%20Object%20Reference) (OtherActor :type Actor%20Object%20Reference) (OtherComp :type Primitive%20Component%20Object%20Reference) (OtherBodyIndex :type Integer))
  ;[0.15 0.15 0.15 0.5] Toggle Player imput on proximity with collision box
  (Rendering|SetVisibility (Variables|Default|GetWidget) false false)
  (if (== (Game|Player|GetPlayerPawn 0) OtherActor)
    (Input|DisableInput (Game|GetPlayerController 0))))

(event OnComponentBeginOverlap(Box)
  (params (OverlappedComponent :type Primitive%20Component%20Object%20Reference) (OtherActor :type Actor%20Object%20Reference) (OtherComp :type Primitive%20Component%20Object%20Reference) (OtherBodyIndex :type Integer) (bFromSweep :type Boolean) (SweepResult :type Hit%20Result%20Structure%20%28by%20ref%29))
  ;[0.15 0.15 0.15 0.5] Toggle Player imput on proximity with collision box
  (Rendering|SetVisibility (Variables|Default|GetWidget) true false)
  (if (== OtherActor (Game|Player|GetPlayerPawn 0))
    (Input|EnableInput (Game|GetPlayerController 0))))

(event Input|KeyboardEvents|Right
  (params (Key :type Key%20Structure :default "None"))
  ;[0.15 0.15 0.15 0.5] Rotate Hour Hand
  (:Pressed
    (Transformation|AddLocalRotation (Variables|Default|GetPresantClock_SmallHand) "-30.000000,0.000000,0.000000" false false)))

(event Input|KeyboardEvents|Left
  (params (Key :type Key%20Structure :default "None"))
  ;[0.15 0.15 0.15 0.5] Rotate Hour Hand
  (:Pressed
    (Transformation|AddLocalRotation (Variables|Default|GetPresantClock_SmallHand) "30.000000,0.000000,0.000000" false false)))

(event Input|KeyboardEvents|E
  (params (Key :type Key%20Structure :default "None"))
  (bind _returnvalue (Game|GetPlayerController 0))
  ;[0.15 0.15 0.15 0.5] Time Menu
  (:Pressed
    (bind _asgi_it (Utilities|Casting|CastToGI_It (Game|GetGameInstance)))
    (if (Variables|/Game/MAIN/GI_It.GI_It_C|GetSecondRound _asgi_it)
      (bind _returnvalue_2 (UserInterface|CreateWidget "/Game/MAIN/Blueprints/Interactable/PresentPuzzle/WBP_PipePuzzle.WBP_PipePuzzle_C" 0 0))
      (UserInterface|Viewport|AddtoViewport _returnvalue_2 0)
      (Variables|/Script/Engine.PlayerController|SetbShowMouseCursor _returnvalue true)
      (Input|SetInputModeGameandUI _returnvalue _returnvalue_2 "DoNotLock" true false)
      (else
        (bind _returnvalue_3 (UserInterface|CreateWidget "/Game/MAIN/Blueprints/Interactable/PresentPuzzle/WBP_BrokenClock.WBP_BrokenClock_C" _returnvalue (Variables|Default|GetLoadingScreenWidget)))
        (UserInterface|Viewport|AddtoViewport _returnvalue_3 0)
        (Input|SetInputModeUIOnly (Game|GetPlayerController 0) _returnvalue_3 "DoNotLock" true)
        (Variables|/Script/Engine.PlayerController|SetbShowMouseCursor (Game|GetPlayerController 0) true)))))

(event Input|KeyboardEvents|Up
  (params (Key :type Key%20Structure :default "None"))
  (bind _presantclock_bighand (Variables|Default|GetPresantClock_BigHand))
  ;[0.15 0.15 0.15 0.5] Rotate Minute hand 1min/5min(shift) per tap
  (:Pressed
    (if (Game|Player|IsInputKeyDown (Game|GetPlayerController 0) "LeftShift")
      (Transformation|AddLocalRotation _presantclock_bighand "-30.000000,0.000000,0.000000" false false)
      (else
        (Transformation|AddLocalRotation _presantclock_bighand "-4.000000,0.000000,0.000000" false false)))))

(event Input|KeyboardEvents|Down
  (params (Key :type Key%20Structure :default "None"))
  (bind _presantclock_bighand (Variables|Default|GetPresantClock_BigHand))
  ;[0.15 0.15 0.15 0.5] Rotate Minute hand 1min/5min(shift) per tap
  (:Pressed
    (if (Game|Player|IsInputKeyDown (Game|GetPlayerController 0) "LeftShift")
      (Transformation|AddLocalRotation _presantclock_bighand "30.000000,0.000000,0.000000" false false)
      (else
        (Transformation|AddLocalRotation _presantclock_bighand "4.000000,0.000000,0.000000" false false)))))

(fn ConstructionScript)
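; BP_ClockFuture is an interactive clock whose hour and minute values the player sets with the arrow keys.
; A collision box enables input on the actor while the player pawn overlaps it and disables it on exit.
; Left and Right adjust hours, while Up and Down adjust minutes, with Left Shift giving larger minute steps.
; Values are clamped rather than wrapped and written straight to separate hour and minute text components.
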(event OnComponentBeginOverlap(Box)
  (params (OverlappedComponent :type Primitive%20Component%20Object%20Reference) (OtherActor :type Actor%20Object%20Reference) (OtherComp :type Primitive%20Component%20Object%20Reference) (OtherBodyIndex :type Integer) (bFromSweep :type Boolean) (SweepResult :type Hit%20Result%20Structure%20%28by%20ref%29))
  ;[0.15 0.15 0.15 0.5] Toggle Player imput on proximity with collision box
  (if (== OtherActor (Game|Player|GetPlayerPawn 0))
    (Input|EnableInput (Game|GetPlayerController 0))))

(event OnComponentEndOverlap(Box)
  (params (OverlappedComponent :type Primitive%20Component%20Object%20Reference) (OtherActor :type Actor%20Object%20Reference) (OtherComp :type Primitive%20Component%20Object%20Reference) (OtherBodyIndex :type Integer))
  ;[0.15 0.15 0.15 0.5] Toggle Player imput on proximity with collision box
  (if (== OtherActor (Game|Player|GetPlayerPawn 0))
    (Input|DisableInput (Game|GetPlayerController 0))))

(event Input|KeyboardEvents|Right
  (params (Key :type Key%20Structure :default "None"))
  ;[0.15 0.15 0.15 0.5] Increase Hour Value
  (:Pressed
    (bind _result (Math|Integer|IncrementInt (Variables|Default|GetHour))
      (:%20%20
        (bind _output_get (Variables|Default|SetHour (Math|Integer|Clamp(Integer) _result 0 24)))
        (Rendering|Components|TextRender|SetText (Variables|Default|GetTR_Hours) (Utilities|Text|ToText(Integer) _output_get false true 2 2))))))

(event Input|KeyboardEvents|Left
  (params (Key :type Key%20Structure :default "None"))
  ;[0.15 0.15 0.15 0.5] Increase Hour Value
  (:Pressed
    (bind _result (Math|Integer|DecrementInt (Variables|Default|GetHour))
      (:%20%20
        (bind _output_get (Variables|Default|SetHour (Math|Integer|Clamp(Integer) _result 0 24)))
        (Rendering|Components|TextRender|SetText (Variables|Default|GetTR_Hours) (Utilities|Text|ToText(Integer) _output_get false true 2 2))))))

(event Input|KeyboardEvents|Up
  (params (Key :type Key%20Structure :default "None"))
  (bind _tr_minutes (Variables|Default|GetTR_Minutes))
  ;[0.15 0.15 0.15 0.5] Increase Minute Value
  (:Pressed
    (if (Game|Player|IsInputKeyDown (Game|GetPlayerController 0) "LeftShift")
      (bind _output_get (Variables|Default|SetMinute (Math|Integer|Clamp(Integer) (+ (Variables|Default|GetMinute) 5) 0 60)))
      (Rendering|Components|TextRender|SetText _tr_minutes (Utilities|Text|ToText(Integer) _output_get false true 2 2))
      (else
        (bind _result (Math|Integer|IncrementInt (Variables|Default|GetMinute))
          (:%20%20
            (bind _output_get_2 (Variables|Default|SetMinute (Math|Integer|Clamp(Integer) _result 0 60)))
            (Rendering|Components|TextRender|SetText _tr_minutes (Utilities|Text|ToText(Integer) _output_get_2 false true 2 2))))))))

(event Input|KeyboardEvents|Down
  (params (Key :type Key%20Structure :default "None"))
  (bind _tr_minutes (Variables|Default|GetTR_Minutes))
  ;[0.15 0.15 0.15 0.5] Increase Minute Value
  (:Pressed
    (if (Game|Player|IsInputKeyDown (Game|GetPlayerController 0) "LeftShift")
      (bind _output_get (Variables|Default|SetMinute (Math|Integer|Clamp(Integer) (- (Variables|Default|GetMinute) 5) 0 60)))
      (Rendering|Components|TextRender|SetText _tr_minutes (Utilities|Text|ToText(Integer) _output_get false true 2 2))
      (else
        (bind _result (Math|Integer|DecrementInt (Variables|Default|GetMinute))
          (:%20%20
            (bind _output_get_2 (Variables|Default|SetMinute (Math|Integer|Clamp(Integer) _result 0 60)))
            (Rendering|Components|TextRender|SetText _tr_minutes (Utilities|Text|ToText(Integer) _output_get_2 false true 2 2))))))))

(fn ConstructionScript)
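; BP_ClockPast is an interactive clock actor, the "past" clock, whose hands the player sets by hand.
; A box overlap enables the actor's input while the player pawn is inside and disables it on exit.
; Left and Right step the hour hand, while Up and Down turn the minute hand, with Left Shift giving larger steps.
; Hands move by relative local rotation, with no time value stored or checked here.
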(event OnComponentBeginOverlap(Box)
  (params (OverlappedComponent :type Primitive%20Component%20Object%20Reference) (OtherActor :type Actor%20Object%20Reference) (OtherComp :type Primitive%20Component%20Object%20Reference) (OtherBodyIndex :type Integer) (bFromSweep :type Boolean) (SweepResult :type Hit%20Result%20Structure%20%28by%20ref%29))
  ;[0.15 0.15 0.15 0.5] Toggle Player imput on proximity with collision box
  (if (== OtherActor (Game|Player|GetPlayerPawn 0))
    (Input|EnableInput (Game|GetPlayerController 0))))

(event OnComponentEndOverlap(Box)
  (params (OverlappedComponent :type Primitive%20Component%20Object%20Reference) (OtherActor :type Actor%20Object%20Reference) (OtherComp :type Primitive%20Component%20Object%20Reference) (OtherBodyIndex :type Integer))
  ;[0.15 0.15 0.15 0.5] Toggle Player imput on proximity with collision box
  (if (== OtherActor (Game|Player|GetPlayerPawn 0))
    (Input|DisableInput (Game|GetPlayerController 0))))

(event Input|KeyboardEvents|Right
  (params (Key :type Key%20Structure :default "None"))
  ;[0.15 0.15 0.15 0.5] Rotate Hour Hand
  (:Pressed
    (Transformation|AddLocalRotation (Variables|Default|GetPastClock_SmallHand) "30.000000,0.000000,0.000000" false false)))

(event Input|KeyboardEvents|Left
  (params (Key :type Key%20Structure :default "None"))
  ;[0.15 0.15 0.15 0.5] Rotate Hour Hand
  (:Pressed
    (Transformation|AddLocalRotation (Variables|Default|GetPastClock_SmallHand) "-30.000000,0.000000,0.000000" false false)))

(event Input|KeyboardEvents|Up
  (params (Key :type Key%20Structure :default "None"))
  (bind _pastclock_bighand (Variables|Default|GetPastClock_BigHand))
  ;[0.15 0.15 0.15 0.5] Rotate Minute hand 1min/5min(shift) per tap
  (:Pressed
    (if (Game|Player|IsInputKeyDown (Game|GetPlayerController 0) "LeftShift")
      (Transformation|AddLocalRotation _pastclock_bighand "30.000000,0.000000,0.000000" false false)
      (else
        (Transformation|AddLocalRotation _pastclock_bighand "4.000000,0.000000,0.000000" false false)))))

(event Input|KeyboardEvents|Down
  (params (Key :type Key%20Structure :default "None"))
  (bind _pastclock_bighand (Variables|Default|GetPastClock_BigHand))
  ;[0.15 0.15 0.15 0.5] Rotate Minute hand 1min/5min(shift) per tap
  (:Pressed
    (if (Game|Player|IsInputKeyDown (Game|GetPlayerController 0) "LeftShift")
      (Transformation|AddLocalRotation _pastclock_bighand "-30.000000,0.000000,0.000000" false false)
      (else
        (Transformation|AddLocalRotation _pastclock_bighand "-4.000000,0.000000,0.000000" false false)))))

(fn ConstructionScript)